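; Parent card actor for a board game that draws a random card matching the active player's current cell type.
; SetCardType maps Divinity, Yokai, Event or Shop cells to a card category, and SetEventCards spawns a random class from that pool.
; The spawned actor's name, type, effect, story and image are copied here, then WBP_Card displays briefly.
; Only Yokai draws call CardEffectActivate, an empty stub in this class.
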(event Custom|SetCardType
  (bind _activeplayer (Class|BPICellRequestReceiver|GetActivePlayer(Message) (Game|GetGameState)))
  (switch Utilities|FlowControl|Switch|SwitchonECellType (Variables|/Game/Path/BP_PathCell.BP_PathCell_C|GetCellType (Variables|/Game/Player/BP_Pion.BP_Pion_C|GetcurrentCell _activeplayer))
    (:NewEnumerator1
      (Variables|Default|SetCardTypes "NewEnumerator2"))
    (:NewEnumerator2
      (Variables|Default|SetCardTypes "NewEnumerator0"))
    (:NewEnumerator3
      (Variables|Default|SetCardTypes "NewEnumerator3"))
    (:NewEnumerator4
      (Variables|Default|SetCardTypes "NewEnumerator1")))
  (CallFunction|SetEventCards)
  (bind _returnvalue (UserInterface|CreateWidget "/Game/Cards/WBP_Card.WBP_Card_C"))
  (UserInterface|Viewport|AddtoViewport _returnvalue 0)
  (Utilities|FlowControl|Delay 5.0)
  (Widget|RemovefromParent _returnvalue))

(event EventBeginPlay)

(event Collision|EventActorBeginOverlap
  (params (OtherActor :type Actor%20Object%20Reference)))

(event EventTick
  (params (DeltaSeconds :type Float%20%28single-precision%29)))

(fn ConstructionScript)

(fn SetEventCards
  (switch Utilities|FlowControl|Switch|SwitchonE_CardType (Variables|Default|GetCardTypes)
    (:NewEnumerator0
      (|YokaiUpdateCard))
    (:NewEnumerator1
      (|CollapseGraph))
    (:NewEnumerator2
      (|CollapseGraph_0))
    (:NewEnumerator3
      (|CollapseGraph_1))))

(fn CardEffectActivate)