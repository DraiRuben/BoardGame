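; BP_Byakko is a divinity card that replaces the active player's dice roll with a one-step move chosen from all paths.
; On activation it waits briefly, marks the cell as used, adds the card to the HUD inventory and binds its click.
; Clicking before rolling or moving enables all paths, clears the current cell, sets path-choice state and hides the dice.
; It then consumes itself by unbinding, removing the widget and destroying the actor.
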(event Custom|TryUse
  (bind _gamestate (CallFunction|GetGamestate))
  (bind _gamestate_2 (CallFunction|GetGamestate))
  (bind _widgetcard (Variables|Default|GetWidgetCard))
  (bind _activeplayer (Default|GetActivePlayer _gamestate_2))
  (if (and (not (Variables|/Game/Systems/BP_Gamestate.BP_Gamestate_C|GetIsActivePlayerMoving _gamestate_2)) (not (Variables|/Game/Player/BP_Pion.BP_Pion_C|GetHasUsedDice _activeplayer)))
    (Default|CallOnPathsAllEnabled _gamestate)
    (bind _activeplayer_2 (Default|GetActivePlayer _gamestate))
    (Variables|/Game/Player/BP_Pion.BP_Pion_C|SetIsInPathChoice _activeplayer_2 true)
    (Variables|/Game/Systems/BP_Gamestate.BP_Gamestate_C|SetIsActivePlayerMoving _gamestate false)
    (Variables|/Game/Player/BP_Pion.BP_Pion_C|SetRemainingMovement _activeplayer_2 1)
    (Variables|/Game/Player/BP_Pion.BP_Pion_C|SetCurrentCell _activeplayer_2 0)
    (Default|SetDiceVisibility (CallFunction|GetDiceHUD) false)
    (Variables|/Game/Player/BP_Pion.BP_Pion_C|SetHasUsedDice _activeplayer_2 true)
    (EventDispatchers|UnbindEventfromOnClickinInventory _widgetcard (delegate Custom|TryUse))
    (Widget|RemovefromParent _widgetcard)
    (Actor|DestroyActor)))

(event EventCardEffectActivate
  (bind _widgetcard (Variables|Default|GetWidgetCard))
  (Utilities|FlowControl|Delay 5.0)
  (bind _activeplayer (Class|BPICellRequestReceiver|GetActivePlayer(Message) (Game|GetGameState)))
  (Variables|/Game/Player/BP_Pion.BP_Pion_C|SetHasUsedCell _activeplayer true)
  (Default|AddtoInventory (CallFunction|GetMainHUD) "NewEnumerator2" _widgetcard)
  (EventDispatchers|BindEventtoOnClickinInventory _widgetcard (delegate Custom|TryUse)))

(fn ConstructionScript
  (|CallParentFunction))