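; Divinity card Blueprint for Ebisu that applies one of two effects when the card effect activates.
; If the divinity amount is at least the number of players, it adds four to the game state's Coins.
; Otherwise it sets the game state's EffectProtect flag and marks the active player as having used their cell.
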(event EventBeginPlay
  (|CallParentFunction) ; This node is disabled and will not be called.\nDrag off pins to build functionality.
)

(event EventCardEffectActivate
  (bind _gamestate (CallFunction|GetGamestate))
  (if (>= (CallFunction|GetDivinityAmount) (Utilities|Array|Length (Variables|/Game/Systems/BP_Gamestate.BP_Gamestate_C|GetPlayers (CallFunction|GetGamestate))))
    (Variables|/Game/Systems/BP_Gamestate.BP_Gamestate_C|SetCoins _gamestate (+ (Variables|/Game/Systems/BP_Gamestate.BP_Gamestate_C|GetCoins _gamestate) 4))
    (else
      (bind _output_get (Variables|Default|SetGamestate (CallFunction|GetGamestate)))
      (Variables|/Game/Systems/BP_Gamestate.BP_Gamestate_C|SetEffectProtect _output_get true)
      (bind _activeplayer (Default|GetActivePlayer _output_get))
      (Variables|/Game/Player/BP_Pion.BP_Pion_C|SetHasUsedCell _activeplayer true))))

(fn ConstructionScript
  (|CallParentFunction))