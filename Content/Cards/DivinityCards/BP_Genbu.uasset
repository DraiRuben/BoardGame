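; Genbu divinity card Blueprint that applies a game-state effect when the card is activated.
; If the divinity amount is at least the player count, it adds coins to the game state.
; Otherwise it rolls the global turn back by one, never below the first, then after a short delay marks the captured active player as having used their cell.
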(event EventBeginPlay
  (|CallParentFunction) ; This node is disabled and will not be called.\nDrag off pins to build functionality.
)

(event EventCardEffectActivate
  (bind _gamestate (CallFunction|GetGamestate))
  (bind _gamestate_2 (CallFunction|GetGamestate))
  ;[0.3125 0 1] faire le if pour le trop de divinité
  ;[0 1 0.6484] if divinity amount
  (if (>= (CallFunction|GetDivinityAmount) (Utilities|Array|Length (Variables|/Game/Systems/BP_Gamestate.BP_Gamestate_C|GetPlayers _gamestate_2)))
    (Variables|/Game/Systems/BP_Gamestate.BP_Gamestate_C|SetCoins _gamestate_2 (+ (Variables|/Game/Systems/BP_Gamestate.BP_Gamestate_C|GetCoins _gamestate_2) 4))
    (else
      ;[0 1 0.2734] Substract 1 at Current Global Turn
      (if (> (Variables|/Game/Systems/BP_Gamestate.BP_Gamestate_C|GetCurrentGlobalTurn _gamestate) 1)
        (Variables|/Game/Systems/BP_Gamestate.BP_Gamestate_C|SetCurrentGlobalTurn _gamestate (- (Variables|/Game/Systems/BP_Gamestate.BP_Gamestate_C|GetCurrentGlobalTurn _gamestate) 1)))
      (bind _activeplayer (Default|GetActivePlayer _gamestate))
      (Utilities|FlowControl|Delay 3.0)
      (Variables|/Game/Player/BP_Pion.BP_Pion_C|SetHasUsedCell _activeplayer true))))

(fn ConstructionScript
  (|CallParentFunction))