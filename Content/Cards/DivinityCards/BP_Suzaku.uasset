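; BP_Suzaku is a divinity card that lets a player add a chosen 1–6 bonus to a dice roll.
; On activation, after a delay, it enters the inventory or grants coins if the divinity count has reached the player count, then marks the cell used.
; Clicking it opens the bonus UI, gated on dice HUD state.
; Selection binds the bonus to the dice-roll event, then immediately destroys the card.
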(event Custom|OnClickInInventory
  (bind _returnvalue (Game|GetPlayerController 0))
  (bind _dicehud (CallFunction|GetDiceHUD))
  (bind _returnvalue_2 (HUD|GetHUD _returnvalue))
  (bind _asbp_main_hud (Utilities|Casting|CastToBP_MainHUD _returnvalue_2))
  (bind _dicebonusmalushud (Variables|/Game/Widgets/Main_UI/BP_MainHUD.BP_MainHUD_C|GetDiceBonusMalusHUD _asbp_main_hud))
  ;[1 0 0.1875] Show Chose Dice
  (Default|GetActivePlayer (CallFunction|GetGamestate))
  (switch Utilities|FlowControl|Switch|SwitchonESlateVisibility (Variables|/Script/UMG.Widget|GetVisibility (Variables|/Game/Widgets/Dice/WBP_RollDice.WBP_RollDice_C|GetButton_Roll _dicehud))
    (:Hidden
      (if (Variables|/Game/Assets/Animation/Dice/BP_DiceAnimation.BP_DiceAnimation_C|GetRoll (Variables|/Game/Player/Dice/BP_Dice.BP_Dice_C|GetDiceAnimation (Variables|/Game/Widgets/Dice/WBP_RollDice.WBP_RollDice_C|GetDice _dicehud)))
        (EventDispatchers|UnbindEventfromOnClickinInventory (Variables|Default|GetWidgetCard) (delegate Custom|OnClickInInventory))
        (Development|PrintString "chose UI")
        (Widget|SetVisibility (Variables|/Game/Widgets/Dice/WBP_RollDice.WBP_RollDice_C|GetButton_Roll (CallFunction|GetDiceHUD)) "Hidden")
        (Default|ShowDiceBonusUI _dicebonusmalushud (Utilities|Array|MakeArray 1 2 3 4 5 6))
        (EventDispatchers|BindEventtoOnDiceBonusSelected _dicebonusmalushud (delegate Custom|OnDiceBonusSelected))))))

(event Custom|OnDiceBonusSelected
  (params (Choice :type Integer))
  (bind _dicehud (CallFunction|GetDiceHUD))
  ;[0.7344 1 0] AddChoice
  (Default|GetActivePlayer (CallFunction|GetGamestate))
  (switch Utilities|FlowControl|Switch|SwitchonESlateVisibility (Variables|/Script/UMG.Widget|GetVisibility (Variables|/Game/Widgets/Dice/WBP_RollDice.WBP_RollDice_C|GetButton_Roll (CallFunction|GetDiceHUD)))
    (:Hidden
      (if (Variables|/Game/Assets/Animation/Dice/BP_DiceAnimation.BP_DiceAnimation_C|GetRoll (Variables|/Game/Player/Dice/BP_Dice.BP_Dice_C|GetDiceAnimation (Variables|/Game/Widgets/Dice/WBP_RollDice.WBP_RollDice_C|GetDice _dicehud)))
        (EventDispatchers|BindEventtoOnDiceRoll _dicehud (delegate Custom|Set%20result))
        (Widget|RemovefromParent (Variables|Default|GetWidgetCard))
        (Actor|DestroyActor)))))

(event Custom|Set%20result
  (params (RollValue :type Integer))
  (bind _dicehud (CallFunction|GetDiceHUD))
  (bind _dice (Variables|/Game/Widgets/Dice/WBP_RollDice.WBP_RollDice_C|GetDice _dicehud))
  ;[1 0.8203 0] Set Result
  (Variables|/Game/Player/Dice/BP_Dice.BP_Dice_C|SetResult _dice (+ (Variables|/Game/Player/Dice/BP_Dice.BP_Dice_C|GetResult _dice) (stale Custom|OnDiceBonusSelected Choice)))
  (Development|PrintString "Dice Used"))

(event EventCardEffectActivate
  (bind _gamestate (CallFunction|GetGamestate))
  (bind _widgetcard (Variables|Default|GetWidgetCard))
  ;[0.3594 1 0] Card effect activated
  (Utilities|FlowControl|Delay 5.0)
  (if (< (CallFunction|GetDivinityAmount) (Utilities|Array|Length (Variables|/Game/Systems/BP_Gamestate.BP_Gamestate_C|GetPlayers _gamestate)))
    (Default|AddtoInventory (CallFunction|GetMainHUD) "NewEnumerator2" _widgetcard)
    (EventDispatchers|BindEventtoOnClickinInventory _widgetcard (delegate Custom|OnClickInInventory))
    (else
      (Variables|/Game/Systems/BP_Gamestate.BP_Gamestate_C|SetCoins _gamestate (+ (Variables|/Game/Systems/BP_Gamestate.BP_Gamestate_C|GetCoins _gamestate) 4))))
  (bind _activeplayer (Default|GetActivePlayer _gamestate))
  (Variables|/Game/Player/BP_Pion.BP_Pion_C|SetHasUsedCell _activeplayer true))

(fn ConstructionScript
  (|CallParentFunction))