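; BP_MaledictionOni is an event card that generates a boss when its effect activates.
; After a five-second delay it calls GenerateBoss on the DisplayCard held by the game state.
; Five seconds later it removes the card widget of the returned boss from its parent and destroys its own actor.
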(event EventBeginPlay
  (|CallParentFunction) ; This node is disabled and will not be called.\nDrag off pins to build functionality.
)

(event EventCardEffectActivate
  (Utilities|FlowControl|Delay 5.0)
  (bind _cardwidget (Default|GenerateBoss (Variables|/Game/Systems/BP_Gamestate.BP_Gamestate_C|GetDisplayCard (CallFunction|GetGamestate))))
  (Utilities|FlowControl|Delay 5.0)
  (Widget|RemovefromParent _cardwidget)
  (Actor|DestroyActor))

(fn ConstructionScript
  (|CallParentFunction))