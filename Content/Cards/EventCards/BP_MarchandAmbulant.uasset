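; Event card for a traveling merchant that opens a shop when its effect activates.
; After a five-second delay, it creates a shop widget for the first player controller, adds it to the viewport and opens it.
; It then adds a small coin bonus to the game state, without waiting for the shop to close.
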(event EventCardEffectActivate
  (bind _gamestate (CallFunction|GetGamestate))
  (Utilities|FlowControl|Delay 5.0)
  (bind _returnvalue (UserInterface|CreateWidget "/Game/Widgets/Items/WBP_Shop.WBP_Shop_C" (Game|GetPlayerController 0)))
  (UserInterface|Viewport|AddtoViewport _returnvalue 0)
  (Default|Open _returnvalue)
  (Variables|/Game/Systems/BP_Gamestate.BP_Gamestate_C|SetCoins _gamestate (+ (Variables|/Game/Systems/BP_Gamestate.BP_Gamestate_C|GetCoins _gamestate) 2)))

(fn ConstructionScript
  (|CallParentFunction))