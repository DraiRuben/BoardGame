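; Saruta-hiko event card Blueprint that advances the game's global turn counter when its effect activates.
; CardEffectActivate does nothing while the GameState's EffectProtect is set.
; Otherwise it plays the event sound, increments CurrentGlobalTurn and marks the active player as having used a cell.
; The graph comment says the turn is decremented, but the logic adds one.
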(event EventBeginPlay
  (|CallParentFunction) ; This node is disabled and will not be called.\nDrag off pins to build functionality.
)

(event EventCardEffectActivate
  (bind _gamestate (CallFunction|GetGamestate))
  ;[0 1 0.2734] Substract 1 at Current Global Turn
  (if (not (Variables|/Game/Systems/BP_Gamestate.BP_Gamestate_C|GetEffectProtect _gamestate))
    (Audio|PlaySound2D "/Game/Assets/Audio/SFX/A_Evenement.A_Evenement" 1.0 1.0 0.0 0 0)
    (Variables|/Game/Systems/BP_Gamestate.BP_Gamestate_C|SetCurrentGlobalTurn _gamestate (+ (Variables|/Game/Systems/BP_Gamestate.BP_Gamestate_C|GetCurrentGlobalTurn _gamestate) 1))
    (bind _activeplayer (Default|GetActivePlayer _gamestate))
    (Variables|/Game/Player/BP_Pion.BP_Pion_C|SetHasUsedCell _activeplayer true)))

(fn ConstructionScript
  (|CallParentFunction))