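; Event card Blueprint for Zennyo Ryuo, which makes the active player skip a turn and hampers movement on following turns.
; On activation it marks the player's cell as used, then after short delays sets the skip flag and binds to the GameState's turn-change event.
; Each turn change gives the newly active player a negative movement modifier, with a counter stopping after one fewer than the player count.
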(event Custom|OnPlayerTurnChange
  (if (< (Variables|Default|GetAmountPlayerDecreased) (- (Utilities|Array|Length (Variables|/Game/Systems/BP_Gamestate.BP_Gamestate_C|GetPlayers (CallFunction|GetGamestate))) 1))
    (Math|Integer|IncrementInt (Variables|Default|GetAmountPlayerDecreased)
      (:%20%20
        (bind _activeplayer (Default|GetActivePlayer (CallFunction|GetGamestate)))
        (Variables|/Game/Player/BP_Pion.BP_Pion_C|SetMovementModifier _activeplayer -2)))))

(event EventCardEffectActivate
  (bind _gamestate (CallFunction|GetGamestate))
  (Development|PrintString "ZennyoRyuo")
  (bind _activeplayer (Default|GetActivePlayer _gamestate))
  (Variables|/Game/Player/BP_Pion.BP_Pion_C|SetHasUsedCell _activeplayer true)
  (Utilities|FlowControl|Delay 1.0)
  (bind _activeplayer_2 (Default|GetActivePlayer _gamestate))
  (Variables|/Game/Player/BP_Pion.BP_Pion_C|SetSkipNextTurn _activeplayer_2 true)
  (Utilities|FlowControl|Delay 0.2)
  (EventDispatchers|BindEventtoOnPlayerTurnChange _gamestate (delegate Custom|OnPlayerTurnChange)))

(fn ConstructionScript
  (|CallParentFunction))