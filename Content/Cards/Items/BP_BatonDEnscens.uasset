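; Incense stick item card that turns on a protection effect when clicked in the inventory.
; One tick after BeginPlay, it binds its activation event to the card widget's inventory click.
; On click, if IsBoss is false, it sets EffectProtect on the game state and unbinds itself, so it triggers only once.
; When IsBoss is true, the click does nothing and the binding stays.
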(event EventBeginPlay
  ;[0 1 0.5078] BeginPlay
  (|CallParentFunction)
  (Utilities|FlowControl|DelayUntilNextTick)
  (EventDispatchers|BindEventtoOnClickinInventory (Variables|Default|GetWidgetCard) (delegate EventCardEffectActivate)))

(event EventCardEffectActivate
  ;[1 0 0.4922] CardEffectActivated
  (if (not (Variables|Default|GetIsBoss))
    (Variables|/Game/Systems/BP_Gamestate.BP_Gamestate_C|SetEffectProtect (CallFunction|GetGamestate) true)
    (EventDispatchers|UnbindEventfromOnClickinInventory (Variables|Default|GetWidgetCard) (delegate EventCardEffectActivate))))

(fn ConstructionScript
  (|CallParentFunction))