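; BP_FilRouge is the Fil Rouge item card, whose effect triggers a dice multi-roll for the active player.
; Activation passes the card's Dice to the card effect, which re-enables dice result sending and starts the multi-roll.
; It then writes the dice result back unchanged and flags the active player's message from the GameState as having used the cell.
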(event Custom|Event%20Card%20Effect
  (params (Dice :type WBP%20Roll%20Dice%20Object%20Reference))
  (bind _diceresult (Variables|Default|GetDiceResult))
  (Variables|/Game/Widgets/Dice/WBP_RollDice.WBP_RollDice_C|SetPauseDiceResultSend Dice false)
  (Default|StartMultiRoll Dice)
  (Variables|/Game/Player/Dice/BP_Dice.BP_Dice_C|SetResult _diceresult (Variables|/Game/Player/Dice/BP_Dice.BP_Dice_C|GetResult _diceresult))
  (bind _activeplayer (Class|BPICellRequestReceiver|GetActivePlayer(Message) (Game|GetGameState)))
  (Variables|/Game/Player/BP_Pion.BP_Pion_C|SetHasUsedCell _activeplayer true))

(event EventBeginPlay)

(event Collision|EventActorBeginOverlap
  (params (OtherActor :type Actor%20Object%20Reference)))

(event EventTick
  (params (DeltaSeconds :type Float%20%28single-precision%29))
  (|CallParentFunction DeltaSeconds) ; This node is disabled and will not be called.\nDrag off pins to build functionality.
)

(event EventCardEffectActivate
  (CallFunction|EventCardEffect (Variables|Default|GetDice)))

(fn ConstructionScript
  (|CallParentFunction))