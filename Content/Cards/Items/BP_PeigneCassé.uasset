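; Item card actor for PeigneCassé (broken comb), a single-use card activated from the inventory.
; One tick after BeginPlay, it binds its activation event to the card widget's inventory click.
; On activation it removes the widget, has the GameState's DisplayCard generate cards from a fixed enum value, then destroys itself.
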(event EventBeginPlay
  (|CallParentFunction)
  (Utilities|FlowControl|DelayUntilNextTick)
  (EventDispatchers|BindEventtoOnClickinInventory (Variables|Default|GetWidgetCard) (delegate EventCardEffectActivate)))

(event EventCardEffectActivate
  (Widget|RemovefromParent (Variables|Default|GetWidgetCard))
  (Default|GenerateCards (Variables|/Game/Systems/BP_Gamestate.BP_Gamestate_C|GetDisplayCard (CallFunction|GetGamestate)) "NewEnumerator0")
  (Actor|DestroyActor))

(fn ConstructionScript
  (|CallParentFunction))