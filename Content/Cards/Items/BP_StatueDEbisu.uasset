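; Ebisu statue item card that adds a fixed bonus to the dice result when clicked in the inventory.
; Once in the inventory, a one-shot Tick check requests dice interruption and binds dice events that enable clicking after a roll and disable it once used.
; Use requires no remaining movement, then releases the interruption and destroys the card.
; Bonus-choice and cancel handlers exist, but nothing here connects them.
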(event Custom|use
  (bind _dicehud (CallFunction|GetDiceHUD))
  (bind _dice (Variables|/Game/Widgets/Dice/WBP_RollDice.WBP_RollDice_C|GetDice _dicehud))
  ;[0.9688 1 0] OnClickInInventory
  (CallFunction|CannotUse)
  (bind _activeplayer (Default|GetActivePlayer (CallFunction|GetGamestate)))
  (if (<= (Variables|/Game/Player/BP_Pion.BP_Pion_C|GetRemainingMovement _activeplayer) 0)
    (Variables|/Game/Dice/BP_Dice.BP_Dice_C|SetResult _dice (+ (Variables|/Game/Dice/BP_Dice.BP_Dice_C|GetResult _dice) 3))
    (Default|RequestDiceInterruptionChange (CallFunction|GetDiceHUD) false)
    (Widget|RemovefromParent (Variables|Default|GetWidgetCard))
    (Audio|PlaySound2D "/Game/Assets/Audio/SFX/A_UtilisationObjet.A_UtilisationObjet" 1.0 1.0 0.0 0 0)
    (Actor|DestroyActor)))

(event Custom|OnDiceBonusSelected
  (params (Choice :type Integer))
  (bind _dicehud (CallFunction|GetDiceHUD))
  (bind _dice (Variables|/Game/Widgets/Dice/WBP_RollDice.WBP_RollDice_C|GetDice _dicehud))
  (Widget|RemovefromParent (Variables|Default|GetWidgetCard))
  (Variables|/Game/Dice/BP_Dice.BP_Dice_C|SetResult _dice (+ (Variables|/Game/Dice/BP_Dice.BP_Dice_C|GetResult _dice) Choice))
  (Default|RequestDiceInterruptionChange (CallFunction|GetDiceHUD) false)
  (Actor|DestroyActor))

(event Custom|CanUse
  (params (RollValue :type Integer))
  (EventDispatchers|BindEventtoOnClickinInventory (Variables|Default|GetWidgetCard) (delegate Custom|OnClickInInventory)))

(event Custom|CannotUse
  (params (Dice%20Value :type Integer))
  (EventDispatchers|UnbindEventfromOnClickinInventory (Variables|Default|GetWidgetCard) (delegate Custom|OnClickInInventory)))

(event Custom|CancelUse
  (Default|RequestDiceInterruptionChange (CallFunction|GetDiceHUD) false)
  (EventDispatchers|UnbindEventfromOnClickinInventory (Variables|Default|GetWidgetCard) (delegate Custom|CancelUse))
  (CallFunction|CanUse)
  (Default|HideDiceBonusUI (CallFunction|GetDiceBonusHUD)))

(event Custom|OnClickInInventory
  (CallFunction|Use))

(event EventBeginPlay
  (|CallParentFunction))

(event EventTick
  (params (DeltaSeconds :type Float%20%28single-precision%29))
  (bind _dicehud (CallFunction|GetDiceHUD))
  (if (Variables|/Game/Cards/WBP_Card.WBP_Card_C|GetIsInInventory (Variables|Default|GetWidgetCard))
    (Utilities|FlowControl|DoOnce false
      (:Completed
        (Default|RequestDiceInterruptionChange (CallFunction|GetDiceHUD) true)
        (EventDispatchers|BindEventtoOnDiceRoll _dicehud (delegate Custom|CanUse))
        (EventDispatchers|BindEventtoOnDiceUsed _dicehud (delegate Custom|CannotUse))))))

(fn ConstructionScript
  (|CallParentFunction))