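; Statue de Daikokuten item card that acts on the dice result when its effect activates.
; Activation runs CardEffect, which clears the dice's send pause flag, then runs two Sequence branches back to back: result plus one, then minus one.
; Each branch continues into shared logic that unpauses result sending and sets HasUsedCell on the active player obtained from the GameState.
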(event Custom|Event%20Card%20Effect
  (params (Dice :type WBP%20Roll%20Dice%20Object%20Reference))
  (bind _dice_result (Variables|Default|GetDice%20Result))
  (bind _dice_result_2 (Variables|Default|GetDice%20Result))
  (Variables|/Game/Widgets/Dice/WBP_RollDice.WBP_RollDice_C|SetPauseDiceResultSend Dice false)
  (Utilities|FlowControl|Sequence
    (:then_0
      (Variables|/Game/Player/Dice/BP_Dice.BP_Dice_C|SetResult _dice_result_2 (+ (Variables|/Game/Player/Dice/BP_Dice.BP_Dice_C|GetResult _dice_result_2) 1)))
    (:then_1
      (Variables|/Game/Player/Dice/BP_Dice.BP_Dice_C|SetResult _dice_result (- (Variables|/Game/Player/Dice/BP_Dice.BP_Dice_C|GetResult _dice_result) 1))))
  (Default|UnpauseDiceResultSend Dice)
  (bind _activeplayer (Class|BPICellRequestReceiver|GetActivePlayer(Message) (Game|GetGameState)))
  (Variables|/Game/Player/BP_Pion.BP_Pion_C|SetHasUsedCell _activeplayer true))

(event EventBeginPlay
  (|CallParentFunction) ; This node is disabled and will not be called.\nDrag off pins to build functionality.
)

(event Collision|EventActorBeginOverlap
  (params (OtherActor :type Actor%20Object%20Reference))
  (|CallParentFunction OtherActor) ; This node is disabled and will not be called.\nDrag off pins to build functionality.
)

(event EventTick
  (params (DeltaSeconds :type Float%20%28single-precision%29))
  (|CallParentFunction DeltaSeconds) ; This node is disabled and will not be called.\nDrag off pins to build functionality.
)

(event EventCardEffectActivate
  (CallFunction|EventCardEffect (Variables|Default|GetDice)))

(fn ConstructionScript
  (|CallParentFunction))