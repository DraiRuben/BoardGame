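; Yokai card actor Bake Kuijira: a timed challenge that awards a talisman if enough movement is rolled within one global turn.
; On activation it removes the card from the list, sets a target of three moves per player, shows the rule in French and listens to dice use.
; Tick checks the accumulated dice total: success signals the yokai beaten, while turn expiry returns the card; both destroy the actor.
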(event Custom|dice%20roll
  (params (Dice%20Value :type Integer))
  ;[0 1 0.8125] compte le nombre de déplacement
  (Variables|Default|SetCurrentMovement (+ Dice%20Value (Variables|Default|GetCurrentMovement)))
  (EventDispatchers|UnbindEventfromOnDiceUsed (CallFunction|GetDiceHUD) (delegate Custom|dice%20roll)))

(event EventBeginPlay
  (|CallParentFunction) ; This node is disabled and will not be called.\nDrag off pins to build functionality.
)

(event EventTick
  (params (DeltaSeconds :type Float%20%28single-precision%29))
  ;[1 0 0.7969] condition de victoire
  (if (!= (CallFunction|GetCurrentTurn) (+ (Variables|Default|GetCurrentTurn) 1))
    (if (>= (Variables|Default|GetCurrentMovement) (Variables|Default|GetMovementAmountToDo))
      (Utilities|FlowControl|DoOnce false
        (:Completed
          (Math|Integer|IncrementInt (Variables|/Game/Systems/BP_Gamestate.BP_Gamestate_C|GetTalismans (.AsBP%20Gamestate (Utilities|Casting|CastToBP_Gamestate (Game|GetGameState))))
            (:%20%20
              (Development|PrintString "+1 talisman")
              (Default|CallYokaiBeaten (CallFunction|GetGamestate))
              (Actor|DestroyActor :!label _label))))))
    (else
      (Utilities|FlowControl|DoOnce false
        (:Completed
          (Development|PrintString "tour fini")
          (Default|AddCardtoList (Variables|/Game/Systems/BP_Gamestate.BP_Gamestate_C|GetDisplayCard (.AsBP%20Gamestate (Utilities|Casting|CastToBP_Gamestate (Game|GetGameState)))) "BP_Bake_Kuijira_C" "NewEnumerator0")
          (goto _label))))))

(event EventCardEffectActivate
  (bind _returnvalue (Game|GetGameState))
  (bind _returnvalue_2 (Game|GetGameState))
  (bind _returnvalue_3 (Game|GetGameState))
  (bind _asbp_gamestate (Utilities|Casting|CastToBP_Gamestate _returnvalue_2))
  (bind _asbp_gamestate_2 (Utilities|Casting|CastToBP_Gamestate _returnvalue))
  (bind _asbp_gamestate_3 (Utilities|Casting|CastToBP_Gamestate _returnvalue_3))
  (bind _players (Variables|/Game/Systems/BP_Gamestate.BP_Gamestate_C|GetPlayers _asbp_gamestate_2))
  (bind _returnvalue_4 (Utilities|Array|Length _players))
  (bind _returnvalue_5 (* _returnvalue_4 3))
  ;[0.9922 1 0] trigger l'effet
  (Default|RemoveCardfromList (Variables|/Game/Systems/BP_Gamestate.BP_Gamestate_C|GetDisplayCard _asbp_gamestate_3) "BP_Bake_Kuijira_C" "NewEnumerator0")
  (EventDispatchers|BindEventtoOnDiceUsed (Variables|/Game/Systems/BP_Gamestate.BP_Gamestate_C|GetDiceHUD _asbp_gamestate_3) (delegate Custom|dice%20roll))
  (Variables|Default|SetMovementAmountToDo _returnvalue_5)
  (Variables|/Game/Cards/BP_ParentCard.BP_ParentCard_C|SetEffectCard (Variables|/Game/Systems/BP_Gamestate.BP_Gamestate_C|GetDisplayCard _asbp_gamestate) (Utilities|Text|ToText(String) (Utilities|String|Append "Après avoir fait 1 tour de jeu, si vous avez fait " (Utilities|String|ToString(Integer) _returnvalue_5) " déplacements ou plus, vous obtenez un talisman.")))
  (Variables|Default|SetCurrentTurn (Variables|/Game/Systems/BP_Gamestate.BP_Gamestate_C|GetCurrentGlobalTurn _asbp_gamestate))
  (bind _activeplayer (Class|BPICellRequestReceiver|GetActivePlayer(Message) _returnvalue_2))
  (Variables|/Game/Player/BP_Pion.BP_Pion_C|SetHasUsedCell _activeplayer true))

(fn ConstructionScript
  (|CallParentFunction))