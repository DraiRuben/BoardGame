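; Yokai card Blueprint for Gashadokuro, resolving a dice-roll challenge against the active player.
; Activation shows the GameState's dice HUD and binds RollDice to its dice-used event.
; A roll of three or less moves the player two steps backwards unless EffectProtect is set; higher rolls call YokaiBeaten.
; Delays pace the result before it marks the cell used, unbinds and clears backward movement.
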(event Custom|RollDice
  (params (Dice%20Value :type Integer))
  (bind _returnvalue (Game|GetGameState))
  (bind _asbp_gamestate (Utilities|Casting|CastToBP_Gamestate _returnvalue))
  ;[0 1 0.9297] condition de victoire
  (if (<= Dice%20Value 3)
    (if (Variables|/Game/Systems/BP_Gamestate.BP_Gamestate_C|GetEffectProtect (CallFunction|GetGamestate))
      _
      (else
        (Utilities|FlowControl|Delay 2.0)
        (bind _activeplayer (Default|GetActivePlayer _asbp_gamestate))
        (Variables|/Game/Player/BP_Pion.BP_Pion_C|SetMoveBackwards _activeplayer true)
        (Variables|/Game/Player/BP_Pion.BP_Pion_C|SetRemainingMovement _activeplayer 2)))
    (else
      (Default|CallYokaiBeaten _asbp_gamestate)))
  (Utilities|FlowControl|Delay 2.0)
  (bind _activeplayer_2 (Class|BPICellRequestReceiver|GetActivePlayer(Message) (Game|GetGameState)))
  (Variables|/Game/Player/BP_Pion.BP_Pion_C|SetHasUsedCell _activeplayer_2 true)
  (EventDispatchers|UnbindEventfromOnDiceUsed (Variables|/Game/Systems/BP_Gamestate.BP_Gamestate_C|GetDiceHUD _asbp_gamestate) (delegate Custom|RollDice))
  (bind _activeplayer_3 (Default|GetActivePlayer _asbp_gamestate))
  (Variables|/Game/Player/BP_Pion.BP_Pion_C|SetMoveBackwards _activeplayer_3 false))

(event EventBeginPlay
  (|CallParentFunction) ; This node is disabled and will not be called.\nDrag off pins to build functionality.
)

(event EventCardEffectActivate
  (bind _returnvalue (Game|GetGameState))
  (bind _asbp_gamestate (Utilities|Casting|CastToBP_Gamestate _returnvalue))
  (bind _dicehud (Variables|/Game/Systems/BP_Gamestate.BP_Gamestate_C|GetDiceHUD _asbp_gamestate))
  ;[0.8984 0 1] trigger l'effet de la carte
  (Default|SetDiceVisibility _dicehud true)
  (EventDispatchers|BindEventtoOnDiceUsed _dicehud (delegate Custom|RollDice)))

(fn ConstructionScript
  (|CallParentFunction))