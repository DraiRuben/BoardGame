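; BP_Hidarugami is a Yokai card Blueprint whose effect depends on a dice roll.
; Activating the effect shows the game state's dice HUD and binds a roll handler, which unbinds itself when the die is used.
; A six or a value below three only prints French messages announcing a next-turn reroll or skipped turn; other values do nothing.
; Logic setting HasUsedCell on the active player is present but unconnected.
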(event Custom|roll
  (params (Dice%20Value :type Integer))
  (EventDispatchers|UnbindEventfromOnDiceUsed (Variables|/Game/Systems/BP_Gamestate.BP_Gamestate_C|GetDiceHUD (.AsBP%20Gamestate (Utilities|Casting|CastToBP_Gamestate (Game|GetGameState)))) (delegate Custom|roll))
  (if (== Dice%20Value 6)
    (Development|PrintString "relancer au prochain tur")
    (elif (< Dice%20Value 3)
      (Development|PrintString "passez votre tour au prochain tour"))))

(event EventBeginPlay
  (|CallParentFunction) ; This node is disabled and will not be called.\nDrag off pins to build functionality.
)

(event EventCardEffectActivate
  (bind _returnvalue (Game|GetGameState))
  (bind _asbp_gamestate (Utilities|Casting|CastToBP_Gamestate _returnvalue))
  (bind _dicehud (Variables|/Game/Systems/BP_Gamestate.BP_Gamestate_C|GetDiceHUD _asbp_gamestate))
  (Default|SetDiceVisibility _dicehud true)
  (EventDispatchers|BindEventtoOnDiceUsed _dicehud (delegate Custom|roll)))

(fn ConstructionScript
  (|CallParentFunction))