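; Nekomata yokai card actor that grants a talisman when at least two yokai are beaten within its turn window.
; On activation it leaves the card list, records the turn, marks the player's cell used after a delay and enters the inventory.
; A gamestate event or input action increments the count.
; Tick checks it during the two-turn window, either awarding and self-destroying or re-listing the card, removing its widget either way.
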(event Custom|OnYokaiBeaten
  ;[0.2656 1 0] when a yokai is beaten add one to the counter
  (Math|Integer|IncrementInt (Variables|Default|GetBeatenYokaiAmount)
    (:%20%20
      (Development|PrintString "yokai beaten"))))

(event Input|EnhancedActionEvents|EnhancedInputActionIA_BeatYokai
  (params (ActionValue :type Boolean) (ElapsedSeconds :type Float%20%28double-precision%29) (TriggeredSeconds :type Float%20%28double-precision%29) (InputAction :type Input%20Action%20Object%20Reference :default "/Game/Inputs/IA_BeatYokai.IA_BeatYokai"))
  (:Started
    ;[0.2656 1 0] when a yokai is beaten add one to the counter
    (Math|Integer|IncrementInt (Variables|Default|GetBeatenYokaiAmount)
      (:%20%20
        (Development|PrintString "yokai beaten")))))

(event EventBeginPlay
  ;[0.03125 0 1] card effect triggered
  (|CallParentFunction) ; This node is disabled and will not be called.\nDrag off pins to build functionality.
)

(event EventCardEffectActivate
  (bind _returnvalue (Game|GetGameState))
  (bind _asbp_gamestate (Utilities|Casting|CastToBP_Gamestate _returnvalue))
  ;[0.03125 0 1] card effect triggered
  (Default|RemoveCardfromList (Variables|/Game/Systems/BP_Gamestate.BP_Gamestate_C|GetDisplayCard (Utilities|GetGamestate)) "BP_Nekomata_C" "NewEnumerator0")
  (EventDispatchers|BindEventtoYokaiBeaten _asbp_gamestate (delegate Custom|OnYokaiBeaten))
  (Variables|Default|SetCurrentTurn (Variables|/Game/Systems/BP_Gamestate.BP_Gamestate_C|GetCurrentGlobalTurn _asbp_gamestate))
  (bind _activeplayer (Default|GetActivePlayer _asbp_gamestate))
  (Utilities|FlowControl|Delay 5.0)
  (Variables|/Game/Player/BP_Pion.BP_Pion_C|SetHasUsedCell _activeplayer true)
  (Default|AddtoInventory (CallFunction|GetMainHUD) "NewEnumerator0" (Variables|Default|GetWidgetCard)))

(event EventTick
  (params (DeltaSeconds :type Float%20%28single-precision%29))
  ;[0.4297 1 0] as long as the two turns are not finished
  (if (<= (Variables|/Game/Systems/BP_Gamestate.BP_Gamestate_C|GetCurrentGlobalTurn (Utilities|GetGamestate)) (+ (Variables|Default|GetCurrentTurn) 2))
    ;[1 0.7266 0] if the number of beaten yokai is greater than or equal to two
    (if (>= (Variables|Default|GetBeatenYokaiAmount) 2)
      ;[1 0.4453 0] win the talisman
      (Math|Integer|IncrementInt (Variables|/Game/Systems/BP_Gamestate.BP_Gamestate_C|GetTalismans (Utilities|GetGamestate))
        (:%20%20
          (Audio|PlaySound2D "/Game/Assets/Audio/SFX/A_Bonus.A_Bonus" 1.0 1.0 0.0 0 0)
          (Development|PrintString "+1 talisman ")
          (Actor|DestroyActor)))
      (else
        ;[0.7578 0 1] put the card back to the deck
        (Default|AddCardtoList (Variables|/Game/Systems/BP_Gamestate.BP_Gamestate_C|GetDisplayCard (Utilities|GetGamestate)) "BP_Nekomata_C" "NewEnumerator0")))
    (Widget|RemovefromParent (Variables|Default|GetWidgetCard))
    (else
      ;[0.5703 1 0] end of round
      (Utilities|FlowControl|DoOnce false
        (:Completed
          (Development|PrintString "turn end"))))))

(fn ConstructionScript
  (|CallParentFunction))