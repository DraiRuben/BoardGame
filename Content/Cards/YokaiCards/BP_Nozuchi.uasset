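; BP_Nozuchi is a Yokai card whose effect makes a three-dice roll that fails if any two results match.
; Activation clears stored results, shows the gamestate's DiceHUD and starts the multi-roll, binding a callback for when it finishes.
; The callback unbinds itself, scans for duplicates and, on failure, blocks coins for one turn.
; It then marks the active player's cell as used; the failure flag is never reset here.
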(event Custom|multiroll
  (params (MultirollResults :type Array%20of%20Integers))
  ;[0.3125 1 0] Multi roll
  (EventDispatchers|UnbindEventfromOnMultirollFinished (Variables|/Game/Systems/BP_Gamestate.BP_Gamestate_C|GetDiceHUD (.AsBP%20Gamestate (Utilities|Casting|CastToBP_Gamestate (Game|GetGameState)))) (delegate Custom|multiroll))
  ;[1 0.8672 0] Checks in the multi rolls results if there are two same result
  (bind _array_element (Utilities|Array|ForEachLoopwithBreak MultirollResults :!label _label)
    (:LoopBody
      (if (Utilities|Array|ContainsItem (Variables|Default|GetRollsResult) _array_element)
        (Development|PrintString "fail")
        (Variables|Default|SetHasFailedMultiroll true)
        (goto _label Break)
        (else
          (Utilities|Array|Add (Variables|Default|GetRollsResult) _array_element))))
    (:Completed
      (if (Variables|Default|GetHasFailedMultiroll)
        (Default|BlockCoinsfor1Turn (CallFunction|GetGamestate))
        (else
          (Development|PrintString "success")))
      (bind _activeplayer (Class|BPICellRequestReceiver|GetActivePlayer(Message) (Game|GetGameState)))
      (Variables|/Game/Player/BP_Pion.BP_Pion_C|SetHasUsedCell _activeplayer true))))

(event EventBeginPlay
  (|CallParentFunction) ; This node is disabled and will not be called.\nDrag off pins to build functionality.
)

(event EventCardEffectActivate
  (bind _returnvalue (Game|GetGameState))
  (bind _asbp_gamestate (Utilities|Casting|CastToBP_Gamestate _returnvalue))
  (bind _dicehud (Variables|/Game/Systems/BP_Gamestate.BP_Gamestate_C|GetDiceHUD _asbp_gamestate))
  ;[0.2891 1 0] Card effect triggered
  (Utilities|Array|Clear (Variables|Default|GetRollsResult))
  (Default|SetDiceVisibility _dicehud true)
  (Default|StartMultiRoll _dicehud 3)
  (EventDispatchers|BindEventtoOnMultirollFinished _dicehud (delegate Custom|multiroll)))

(fn ConstructionScript
  (|CallParentFunction))