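; Shishi yokai card that offers to trade one of the player's inventory object cards for protection when its effect triggers.
; After a delay, it opens an exchange widget if the HUD's object scroll holds any cards.
; Accepting removes a random object card, sets the GameState's protect flag, calls yokai beaten and plays a bonus sound.
; Accepting, refusing or having no cards marks the active player's cell as used.
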(event Custom|OnTradeAccepted
  (bind _gamestate (CallFunction|GetGamestate))
  ;[1 0.5859 0] When the trade is accepted
  (Widget|RemovefromParent (Utilities|GetRandomObjectCard))
  (Variables|/Game/Systems/BP_Gamestate.BP_Gamestate_C|SetEffectProtect _gamestate true)
  (Default|CallYokaiBeaten _gamestate)
  (Audio|PlaySound2D "/Game/Assets/Audio/SFX/A_Bonus.A_Bonus" 1.0 1.0 0.0 0 0)
  ;[0.3594 0 1] Next player
  (bind _activeplayer (Default|GetActivePlayer (CallFunction|GetGamestate)))
  (Variables|/Game/Player/BP_Pion.BP_Pion_C|SetHasUsedCell _activeplayer true))

(event Custom|OnTradeRefuse
  ;[0.3594 0 1] Next player
  (bind _activeplayer (Default|GetActivePlayer (CallFunction|GetGamestate)))
  (Variables|/Game/Player/BP_Pion.BP_Pion_C|SetHasUsedCell _activeplayer true))

(event EventBeginPlay
  (|CallParentFunction) ; This node is disabled and will not be called.\nDrag off pins to build functionality.
)

(event EventCardEffectActivate
  ;[0 0.1797 1] Card effect triggered
  (Utilities|FlowControl|Delay 5.0)
  (if (> (Class|PanelWidget|GetChildrenCount (Variables|/Game/Widgets/GameUI/WBP_Inventory.WBP_Inventory_C|GetObjectCardScroll (Variables|/Game/Widgets/GameUI/WBP_MainUI.WBP_MainUI_C|GetW_INV_Object (CallFunction|GetMainHUD)))) 0)
    (bind _returnvalue (UserInterface|CreateWidget "/Game/Widgets/Yokais/WBP_ShishiExchange.WBP_ShishiExchange_C"))
    (UserInterface|Viewport|AddtoViewport _returnvalue 0)
    (EventDispatchers|BindEventtoAcceptTrade _returnvalue (delegate Custom|OnTradeAccepted))
    (EventDispatchers|BindEventtoRefuseTrade _returnvalue (delegate Custom|OnTradeRefuse))
    (else
      ;[0.3594 0 1] Next player
      (bind _activeplayer (Default|GetActivePlayer (CallFunction|GetGamestate)))
      (Variables|/Game/Player/BP_Pion.BP_Pion_C|SetHasUsedCell _activeplayer true))))

(fn ConstructionScript
  (|CallParentFunction))