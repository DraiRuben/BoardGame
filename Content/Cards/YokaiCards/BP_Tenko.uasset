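; BP_Tenko is a yokai card whose effect rolls one die per player to win a talisman, provided none shows 1 or 6.
; Activation starts a multi-roll on the dice HUD and handles its finished event.
; As wired, the first result decides: a safe value increments the game state's talismans, plays a bonus sound and calls YokaiBeaten.
; Either outcome sets HasUsedCell on the active player.
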(event Custom|MultiRoll
  (params (MultirollResults :type Array%20of%20Integers))
  (bind _gamestate (CallFunction|GetGamestate))
  ;[1 0 0.6562] Multi roll
  (EventDispatchers|UnbindEventfromOnMultirollFinished (CallFunction|GetDiceHUD) (delegate Custom|MultiRoll))
  ;[0 0.6484 1] Checks if any result of the multi roll is 1 or 6
  (bind _array_element (Utilities|Array|ForEachLoopwithBreak MultirollResults :!label _label)
    (:LoopBody
      (if (or (== _array_element 1) (== _array_element 6))
        (goto _label Break)
        (else
          ;[0.3594 0 1] Add talismans
          (Math|Integer|IncrementInt (Utilities|GetTalismans)
            (:%20%20
              (Audio|PlaySound2D "/Game/Assets/Audio/SFX/A_Bonus.A_Bonus" 1.0 1.0 0.0 0 0)
              (Development|PrintString "+1 talisman")
              (Default|CallYokaiBeaten _gamestate))))))
    (:Completed
      _))
  ;[1 0 0.8672] Next player
  (bind _activeplayer (Default|GetActivePlayer _gamestate))
  (Variables|/Game/Player/BP_Pion.BP_Pion_C|SetHasUsedCell _activeplayer true)
  (goto _label Break))

(event EventBeginPlay
  (bind _returnvalue (Utilities|GetNbPlayers))
  ;[1 0.3984 0] Set the amount of dice to roll
  (|CallParentFunction)
  (Development|PrintString (Utilities|String|ToString(Integer) _returnvalue))
  (Variables|Default|SetEffectCard (Utilities|Text|ToText(String) (Utilities|String|Append "Lancez " (Utilities|String|ToString(Integer) _returnvalue) " dés, si aucun des résultats n'est 1 ou 6, vous gagnez un talisman"))))

(event EventCardEffectActivate
  (bind _dicehud (CallFunction|GetDiceHUD))
  ;[0.4766 0 1] Card effect triggered
  (Default|SetDiceVisibility _dicehud true)
  (Default|StartMultiRoll _dicehud (Utilities|GetNbPlayers))
  (EventDispatchers|BindEventtoOnMultirollFinished _dicehud (delegate Custom|MultiRoll)))

(fn ConstructionScript
  (|CallParentFunction))