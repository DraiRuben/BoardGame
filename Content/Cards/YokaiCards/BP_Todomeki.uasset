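; Todomeki Yokai card that demands 10 coins from the players or sends the active player back to the first cell.
; After a delay, sufficient coins open a pay widget: accepting deducts coins and calls the Yokai-beaten event.
; Refusal or insufficient coins teleports the player with a malus sound, unless EffectProtect is consumed instead.
; Outcomes mark the active player's cell as used, with coins and protection read from the GameState.
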(event Custom|OnTradeAccepted
  (bind _gamestate (CallFunction|GetGamestate))
  ;[1 0.6797 0] If trade accepted pay the 10 coins
  (EventDispatchers|UnbindEventfromAcceptTrade (stale EventCardEffectActivate _returnvalue) (delegate Custom|OnTradeAccepted))
  (Default|CallYokaiBeaten _gamestate)
  (Variables|/Game/Systems/BP_Gamestate.BP_Gamestate_C|SetCoins _gamestate (- (Variables|/Game/Systems/BP_Gamestate.BP_Gamestate_C|GetCoins _gamestate) 10))
  ;[0.5 0 1] next player
  (Widget|RemovefromParent (stale EventCardEffectActivate _returnvalue))
  (bind _activeplayer (Default|GetActivePlayer (CallFunction|GetGamestate)))
  (Variables|/Game/Player/BP_Pion.BP_Pion_C|SetHasUsedCell _activeplayer true))

(event Custom|OnTradeRefused
  (bind _gamestate (CallFunction|GetGamestate))
  (bind _gamestate_2 (CallFunction|GetGamestate))
  (bind _firstcell (Variables|/Game/Systems/BP_Gamestate.BP_Gamestate_C|GetFirstCell _gamestate))
  (bind _returnvalue (Transformation|GetActorLocation _firstcell))
  (bind (_x _y _z) (Math|Vector|BreakVector _returnvalue))
  (bind _returnvalue_2 (+ _z 8e+01))
  (bind _returnvalue_3 (Math|Vector|MakeVector _x _y _returnvalue_2))
  ;[0.875 0 1] If trade refused tp to the spawn
  (if (Variables|/Game/Systems/BP_Gamestate.BP_Gamestate_C|GetEffectProtect _gamestate_2)
    (Variables|/Game/Systems/BP_Gamestate.BP_Gamestate_C|SetEffectProtect _gamestate_2 false)
    (else
      (Audio|PlaySound2D "/Game/Assets/Audio/SFX/A_Malus.A_Malus" 1.0 1.0 0.0 0 0)
      (EventDispatchers|UnbindEventfromRefuseTrade (stale EventCardEffectActivate _returnvalue) (delegate Custom|OnTradeRefused))
      (bind _activeplayer (Default|GetActivePlayer _gamestate))
      (Variables|/Game/Player/BP_Pion.BP_Pion_C|SetCurrentCell _activeplayer _firstcell)
      (Variables|/Game/Player/BP_Pion.BP_Pion_C|SetStartPos _activeplayer _returnvalue_3)
      (Transformation|SetActorLocation _activeplayer _returnvalue_3 false true)))
  ;[0.5 0 1] next player
  (Widget|RemovefromParent (stale EventCardEffectActivate _returnvalue))
  (bind _activeplayer_2 (Default|GetActivePlayer (CallFunction|GetGamestate)))
  (Variables|/Game/Player/BP_Pion.BP_Pion_C|SetHasUsedCell _activeplayer_2 true))

(event EventBeginPlay
  (|CallParentFunction))

(event EventCardEffectActivate
  (bind _gamestate (CallFunction|GetGamestate))
  ;[0 0.625 1] Card effect triggered
  (Utilities|FlowControl|Delay 5.0)
  ;[1 0.9375 0] If the players have at least 10 coins
  (if (>= (Variables|/Game/Systems/BP_Gamestate.BP_Gamestate_C|GetCoins (CallFunction|GetGamestate)) 10)
    ;[0.5 1 0] if has 10 coins
    (Development|PrintString "Continue")
    (bind _returnvalue (UserInterface|CreateWidget "/Game/Widgets/Yokais/WBP_TodomekiPay.WBP_TodomekiPay_C"))
    (UserInterface|Viewport|AddtoViewport _returnvalue 0)
    (EventDispatchers|BindEventtoAcceptTrade _returnvalue (delegate Custom|OnTradeAccepted))
    (EventDispatchers|BindEventtoRefuseTrade _returnvalue (delegate Custom|OnTradeRefused))
    (else
      ;[0 1 0.3203] Tp to start if hasn't 10 coins
      (if (Variables|/Game/Systems/BP_Gamestate.BP_Gamestate_C|GetEffectProtect _gamestate)
        (Variables|/Game/Systems/BP_Gamestate.BP_Gamestate_C|SetEffectProtect _gamestate false)
        (else
          (Development|PrintString "TP Start")
          (CallFunction|OnTradeRefused)))
      ;[0.5 0 1] next player
      (bind _activeplayer (Default|GetActivePlayer (CallFunction|GetGamestate)))
      (Variables|/Game/Player/BP_Pion.BP_Pion_C|SetHasUsedCell _activeplayer true))))

(event EventTick
  (params (DeltaSeconds :type Float%20%28single-precision%29)))

(fn ConstructionScript
  (|CallParentFunction))