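; Yokai card Blueprint for Todomeki, whose effect is a coin check against the player's progress.
; On CardEffectActivate it reads Coins from BP_Gamestate and, at ten or more, calls YokaiBeaten on the game state.
; Below that threshold it only prints a "TP Start" debug string, with no penalty logic in this file.
; BeginPlay and construction defer to the parent class.
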(event EventBeginPlay
  (|CallParentFunction))

(event EventCardEffectActivate
  (bind _returnvalue (Game|GetGameState))
  (bind _asbp_gamestate (Utilities|Casting|CastToBP_Gamestate _returnvalue))
  (Variables|Default|SetAs%20BP%20Gamestate _asbp_gamestate)
  (if (>= (Variables|/Game/Systems/BP_Gamestate.BP_Gamestate_C|GetCoins (Variables|Default|GetAs%20BP%20Gamestate)) 10)
    (Development|PrintString "Continue")
    (Default|YokaiBeaten _asbp_gamestate)
    (else
      (Development|PrintString "TP Start"))))

(event EventTick
  (params (DeltaSeconds :type Float%20%28single-precision%29)))

(fn ConstructionScript
  (|CallParentFunction))