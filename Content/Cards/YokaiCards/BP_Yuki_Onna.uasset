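; Yuki-Onna yokai card that challenges the active player to a two-dice roll.
; On activation it shows the gamestate's DiceHUD, starts the multi-roll and binds a one-shot handler to its finished event.
; The handler adds the dice to DiceResult: above 9 reports the yokai beaten, otherwise a protection effect is consumed or the player skips their next turn.
; Either outcome then flags the active player's cell as used.
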(event Custom|MultiRoll
  (params (MultirollResults :type Array%20of%20Integers))
  (bind _gamestate (CallFunction|GetGamestate))
  ;[0 0.8125 1] Multi roll
  (for _array_element MultirollResults
    ;[0 0.4609 1] Checks if the total dice result if greater than 9
    (Variables|Default|SetDiceResult (+ _array_element (Variables|Default|GetDiceResult))))
  (EventDispatchers|UnbindEventfromOnMultirollFinished (Variables|/Game/Systems/BP_Gamestate.BP_Gamestate_C|GetDiceHUD (.AsBP%20Gamestate (Utilities|Casting|CastToBP_Gamestate (Game|GetGameState)))) (delegate Custom|MultiRoll))
  (if (> (Variables|Default|GetDiceResult) 9)
    ;[0 1 0.4844] success
    (Development|PrintString "success")
    (Default|CallYokaiBeaten _gamestate)
    (else
      ;[0 1 0.9297] Skip Turn
      (if (Variables|/Game/Systems/BP_Gamestate.BP_Gamestate_C|GetEffectProtect _gamestate)
        (Variables|/Game/Systems/BP_Gamestate.BP_Gamestate_C|SetEffectProtect _gamestate false)
        (else
          (Audio|PlaySound2D "/Game/Assets/Audio/SFX/A_Malus.A_Malus" 1.0 1.0 0.0 0 0)
          (bind _activeplayer (Default|GetActivePlayer (CallFunction|GetGamestate)))
          (Variables|/Game/Player/BP_Pion.BP_Pion_C|SetSkipNextTurn _activeplayer true)))))
  ;[0.6641 0 1] Next player
  (bind _activeplayer_2 (Class|BPICellRequestReceiver|GetActivePlayer(Message) (Game|GetGameState)))
  (Variables|/Game/Player/BP_Pion.BP_Pion_C|SetHasUsedCell _activeplayer_2 true))

(event EventBeginPlay
  (|CallParentFunction) ; This node is disabled and will not be called.\nDrag off pins to build functionality.
)

(event EventCardEffectActivate
  (bind _returnvalue (Game|GetGameState))
  (bind _asbp_gamestate (Utilities|Casting|CastToBP_Gamestate _returnvalue))
  (bind _dicehud (Variables|/Game/Systems/BP_Gamestate.BP_Gamestate_C|GetDiceHUD _asbp_gamestate))
  ;[0.125 1 0] Card effect triggered
  (Default|SetDiceVisibility _dicehud true)
  (Default|StartMultiRoll _dicehud 2)
  (EventDispatchers|BindEventtoOnMultirollFinished _dicehud (delegate Custom|MultiRoll)))

(fn ConstructionScript
  (|CallParentFunction))