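; BP_Dice is the dice controller, which spawns a dice animation actor and exposes the rolled Result.
; On BeginPlay it spawns BP_DiceAnimation at one of the first two spawn locations, picked at random, with a slightly randomized rotation.
; Each Tick copies the animation's result into its own, unless debug mode is on.
; Debug input actions force the Result from the input value or return control to the animation.
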(event Input|EnhancedActionEvents|EnhancedInputActionIA_DebugDice
  (params (ActionValue :type Float%20%28double-precision%29) (ElapsedSeconds :type Float%20%28double-precision%29) (TriggeredSeconds :type Float%20%28double-precision%29) (InputAction :type Input%20Action%20Object%20Reference :default "/Game/Inputs/IA_DebugDice.IA_DebugDice"))
  ;[0.4766 1 0] Debug Dice
  (Variables|Default|SetResult (Math|Float|Truncate ActionValue))
  (Variables|Default|SetIsInDebugMode true))

(event Input|EnhancedActionEvents|EnhancedInputActionIA_StopDiceDebug
  (params (ActionValue :type Boolean) (ElapsedSeconds :type Float%20%28double-precision%29) (TriggeredSeconds :type Float%20%28double-precision%29) (InputAction :type Input%20Action%20Object%20Reference :default "/Game/Inputs/IA_StopDiceDebug.IA_StopDiceDebug"))
  (Variables|Default|SetIsInDebugMode false))

(event EventBeginPlay
  (bind _returnvalue (Math|Random|RandomFloat))
  ;[1 0 0.3516] Instantiate Dice Animation
  (bind _returnvalue_2 (Game|SpawnActorfromClass "/Game/Dice/BP_DiceAnimation.BP_DiceAnimation_C" (Math|Transform|MakeTransform (Utilities|Array|Get(acopy) (Variables|Default|GetSpawnLocations) (Math|Random|RandomInteger 2)) (Math|Rotator|MakeRotator _returnvalue _returnvalue _returnvalue)) "Undefined" "MultiplyWithRoot" 0 0))
  (Variables|Default|SetDiceAnimation _returnvalue_2))

(event EventTick
  (params (DeltaSeconds :type Float%20%28single-precision%29))
  ;[0 0.0625 1] Set Dice Result
  (if (not (Variables|Default|GetIsInDebugMode))
    (Variables|Default|SetResult (Variables|/Game/Dice/BP_DiceAnimation.BP_DiceAnimation_C|GetResult (Variables|Default|GetDiceAnimation)))))

(fn ConstructionScript)