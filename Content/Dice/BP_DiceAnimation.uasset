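; Physics-driven dice actor that animates a roll and detects which face it lands on.
; A roll moves the die to a random spawn location, then launches it upward toward the active player with random spin.
; After a short delay, Tick watches for velocity to drop near zero and notifies the game state's DiceHUD that the roll finished.
; Six overlap components, one per face, set the Result value.
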(event OnComponentBeginOverlap(two)
  (params (OverlappedComponent :type Primitive%20Component%20Object%20Reference) (OtherActor :type Actor%20Object%20Reference) (OtherComp :type Primitive%20Component%20Object%20Reference) (OtherBodyIndex :type Integer) (bFromSweep :type Boolean) (SweepResult :type Hit%20Result%20Structure%20%28by%20ref%29))
  ;[0.5234 0 1] Detect Result
  (Variables|Default|SetResult 2))

(event OnComponentBeginOverlap(four)
  (params (OverlappedComponent :type Primitive%20Component%20Object%20Reference) (OtherActor :type Actor%20Object%20Reference) (OtherComp :type Primitive%20Component%20Object%20Reference) (OtherBodyIndex :type Integer) (bFromSweep :type Boolean) (SweepResult :type Hit%20Result%20Structure%20%28by%20ref%29))
  ;[0.5234 0 1] Detect Result
  (Variables|Default|SetResult 4))

(event OnComponentBeginOverlap(three)
  (params (OverlappedComponent :type Primitive%20Component%20Object%20Reference) (OtherActor :type Actor%20Object%20Reference) (OtherComp :type Primitive%20Component%20Object%20Reference) (OtherBodyIndex :type Integer) (bFromSweep :type Boolean) (SweepResult :type Hit%20Result%20Structure%20%28by%20ref%29))
  ;[0.5234 0 1] Detect Result
  (Variables|Default|SetResult 3))

(event OnComponentBeginOverlap(one)
  (params (OverlappedComponent :type Primitive%20Component%20Object%20Reference) (OtherActor :type Actor%20Object%20Reference) (OtherComp :type Primitive%20Component%20Object%20Reference) (OtherBodyIndex :type Integer) (bFromSweep :type Boolean) (SweepResult :type Hit%20Result%20Structure%20%28by%20ref%29))
  ;[0.5234 0 1] Detect Result
  (Variables|Default|SetResult 1))

(event OnComponentBeginOverlap(six)
  (params (OverlappedComponent :type Primitive%20Component%20Object%20Reference) (OtherActor :type Actor%20Object%20Reference) (OtherComp :type Primitive%20Component%20Object%20Reference) (OtherBodyIndex :type Integer) (bFromSweep :type Boolean) (SweepResult :type Hit%20Result%20Structure%20%28by%20ref%29))
  ;[0.5234 0 1] Detect Result
  (Variables|Default|SetResult 6))

(event OnComponentBeginOverlap(five)
  (params (OverlappedComponent :type Primitive%20Component%20Object%20Reference) (OtherActor :type Actor%20Object%20Reference) (OtherComp :type Primitive%20Component%20Object%20Reference) (OtherBodyIndex :type Integer) (bFromSweep :type Boolean) (SweepResult :type Hit%20Result%20Structure%20%28by%20ref%29))
  ;[0.5234 0 1] Detect Result
  (Variables|Default|SetResult 5))

(event Custom|roll%20dice
  (bind _returnvalue (Math|Random|RandomFloatinRange 1e+01 2e+01))
  ;[0 0.5078 1] Roll Dice
  (Transformation|SetActorLocation (Utilities|Array|Get(acopy) (Variables|Default|GetSpawnLocations) (Math|Random|RandomIntegerinRange 0 1)) false false)
  (if (not (Variables|Default|GetRoll))
    (Variables|Default|SetRandomDice (Variables|/Game/Dice/BP_Dice.BP_Dice_C|GetResult (Variables|/Game/Widgets/Dice/WBP_RollDice.WBP_RollDice_C|GetDice (Variables|/Game/Systems/BP_Gamestate.BP_Gamestate_C|GetDiceHUD (.AsBP%20Gamestate (Utilities|Casting|CastToBP_Gamestate (Game|GetGameState)))))))
    (bind _activeplayer (Default|GetActivePlayer (CallFunction|GetGamestate)))
    (Physics|AddImpulse (Variables|Default|GetOBJ) (* (+ (- (Transformation|GetActorLocation _activeplayer) (Transformation|GetActorLocation)) "0.000000,0.000000,1000.000000") 0.5) "None" true)
    (Class|PrimitiveComponent|AddAngularImpulseinRadians (Variables|Default|GetOBJ) (Math|Vector|MakeVector _returnvalue _returnvalue 0.0) "None" true)
    (Utilities|FlowControl|Delay 0.2)
    (Variables|Default|SetRoll true)))

(event Custom|TryFinishRoll
  (bind _gamestate (CallFunction|GetGamestate))
  (bind _dicehud (Variables|/Game/Systems/BP_Gamestate.BP_Gamestate_C|GetDiceHUD _gamestate))
  ;[1 0.09375 0] Try Finish Roll
  (if (< (Math|Vector|VectorLength (Transformation|GetVelocity)) 5.0)
    (Utilities|IsValid _dicehud
      (:Is%20Valid
        (Default|FinishedRoll _dicehud)
        (Variables|Default|SetRoll false)))))

(event EventTick
  (params (DeltaSeconds :type Float%20%28single-precision%29))
  ;[1 0 0.9375] chose dice
  (if (Variables|Default|GetRoll)
    (CallFunction|TryFinishRoll)))

(fn ConstructionScript)