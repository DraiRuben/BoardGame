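; Board-game path cell that links to following and previous cells and applies its effect when used: coins, or setting the display card's type for Divinity, Yokai, Event and Shop.
; On BeginPlay the first cell registers with the GameState, and each cell back-links its connected cells.
; At forks, RequestNextCell highlights the options by material swap; clicking one sets the active player's current cell and disables choice mode through the GameState.
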(event OnClicked(StaticMesh)
  (params (TouchedComponent :type Primitive%20Component%20Object%20Reference) (ButtonPressed :type Key%20Structure :default "None"))
  (bind _returnvalue (Game|GetGameState))
  ;[0 0.4609 1] Tell player what's the next cell for path select
  (if (Variables|Default|GetIsInPathChoiceMode)
    (bind _activeplayer (Class|BPICellRequestReceiver|GetActivePlayer(Message) _returnvalue))
    (Variables|/Game/Player/BP_Pion.BP_Pion_C|SetCurrentCell _activeplayer self)
    (Class|BPICellRequestReceiver|DisablePathChoice(Message) _returnvalue)))

(event Custom|DisableChoiceMode
  (Rendering|Material|SetMaterial (Variables|Default|GetStaticMesh) 0 "/Game/StarterContent/Materials/M_CobbleStone_Pebble.M_CobbleStone_Pebble")
  (Variables|Default|SetIsInPathChoiceMode false))

(event EventBeginPlay
  (bind _returnvalue (Game|GetGameState))
  (bind _asbp_gamestate (Utilities|Casting|CastToBP_Gamestate _returnvalue))
  (EventDispatchers|BindEventtoOnPathChoiceModeDisabled _asbp_gamestate (delegate Custom|DisableChoiceMode))
  (if (Variables|Default|GetIsFirstCell)
    (Variables|/Game/Systems/BP_Gamestate.BP_Gamestate_C|SetFirstCell _asbp_gamestate self))
  (Utilities|FlowControl|DelayUntilNextTick)
  (for _array_element (Variables|Default|GetConnectedCells)
    (Variables|BP_PathCell_C|SetPreviousCell _array_element self)))

(fn ConstructionScript)

(fn EnablePathChoiceMode
  (params (Enabled :type Boolean))
  (bind _staticmesh (Variables|Default|GetStaticMesh))
  (bind _output_get (Variables|Default|SetIsInPathChoiceMode Enabled))
  (if _output_get
    (Rendering|Material|SetMaterial _staticmesh 0 "/Game/StarterContent/Blueprints/Assets/M_LightStage_Skybox_HDRI.M_LightStage_Skybox_HDRI")
    (else
      (Rendering|Material|SetMaterial _staticmesh 0 "/Game/StarterContent/Materials/M_CobbleStone_Pebble.M_CobbleStone_Pebble")))
  (return))

(fn UseCell
  (bind _returnvalue (Game|GetGameState))
  (bind _asbp_gamestate (Utilities|Casting|CastToBP_Gamestate _returnvalue))
  (LocalVariables|SetGameState _asbp_gamestate)
  (Variables|Default|SetCardRef (Variables|/Game/Systems/BP_Gamestate.BP_Gamestate_C|GetDisplayCard _asbp_gamestate))
  (switch Utilities|FlowControl|Switch|SwitchonECellType (Variables|Default|GetCellType)
    (:NewEnumerator0
      (Variables|/Game/Systems/BP_Gamestate.BP_Gamestate_C|SetCoins (LocalVariables|GetGameState) (+ (Variables|/Game/Systems/BP_Gamestate.BP_Gamestate_C|GetCoins (LocalVariables|GetGameState)) (Variables|Default|GetCoinGain)))
      (bind _activeplayer (Default|GetActivePlayer (LocalVariables|GetGameState)))
      (Variables|/Game/Player/BP_Pion.BP_Pion_C|SetHasUsedCell _activeplayer true)
      (return))
    (:NewEnumerator1
      _)
    (:NewEnumerator2
      _)
    (:NewEnumerator3
      _)
    (:NewEnumerator4
      _))
  (Default|SetCardType (Variables|Default|GetCardRef)))

(fn RequestNextCell
  (params (Backwards? :type Boolean))
  (if Backwards?
    (return (Variables|Default|GetPreviousCell))
    (elif (> (Utilities|Array|Length (Variables|Default|GetConnectedCells)) 1)
      (for _array_element (Variables|Default|GetConnectedCells)
        (CallFunction|EnablePathChoiceMode _array_element true))
      (return 0)
      (else
        (return (Utilities|Array|Get(acopy) (Variables|Default|GetConnectedCells)))))))