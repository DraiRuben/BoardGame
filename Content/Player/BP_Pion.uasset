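; Board game pawn that moves cell by cell after a dice roll from the GameState's dice HUD.
; Tick drives movement, asking each cell for the next and pausing at path choices when none is returned.
; Two timelines lerp each step and add a vertical hop.
; At zero remaining movement it triggers the cell once, then requests turn end once HasUsedCell is set; SkipNextTurn ends the turn directly.
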(event Custom|BindToDice
  (params (Bind? :type Boolean))
  (bind _returnvalue (Game|GetGameState))
  (bind _asbp_gamestate (Utilities|Casting|CastToBP_Gamestate _returnvalue))
  (bind _dicehud (Variables|/Game/Systems/BP_Gamestate.BP_Gamestate_C|GetDiceHUD _asbp_gamestate))
  ;[0 0.9297 1] Dice usage
  (if Bind?
    (EventDispatchers|BindEventtoOnDiceUsed _dicehud (delegate Custom|ReceiveDiceUse))
    (else
      (EventDispatchers|UnbindEventfromOnDiceUsed _dicehud (delegate Custom|ReceiveDiceUse)))))

(event Custom|ReceiveDiceUse
  (params (Dice%20Value :type Integer))
  ;[0 0.9297 1] Dice usage
  (Variables|Movement|SetRemainingMovement Dice%20Value)
  (Variables|TurnState|SetHasUsedDice true)
  (EventDispatchers|UnbindEventfromOnDiceUsed (Variables|/Game/Systems/BP_Gamestate.BP_Gamestate_C|GetDiceHUD (.AsBP%20Gamestate (Utilities|Casting|CastToBP_Gamestate (Game|GetGameState)))) (delegate Custom|ReceiveDiceUse)))

(event EventBeginPlay
  (bind _currentcell (Variables|Movement|GetCurrentCell))
  (bind _returnvalue (Transformation|GetActorLocation _currentcell))
  (bind _returnvalue_2 (+ _returnvalue "0.000000,0.000000,88.000000"))
  ;[0.3594 1 0] initial position
  (Utilities|FlowControl|DelayUntilNextTick)
  (Transformation|SetActorLocation _returnvalue_2 false false)
  (Variables|Movement|SetStartPos _returnvalue_2))

(event EventTick
  (params (DeltaSeconds :type Float%20%28single-precision%29))
  (bind _returnvalue (Game|GetGameState))
  (bind _asbp_gamestate (Utilities|Casting|CastToBP_Gamestate _returnvalue))
  ;[0.4297 1 0] pion movement
  (if (and (Variables|TurnState|GetIsActivePlayer) (Variables|TurnState|GetHasUsedDice))
    (Utilities|FlowControl|Delay 0.7)
    (if (> (Variables|Movement|GetRemainingMovement) 0)
      (Utilities|IsValid (Variables|Movement|GetCurrentCell)
        (:Is%20Valid
          (if (Variables|TurnState|GetIsInPathChoice)
            (Variables|Movement|SetEndPos (Transformation|GetActorLocation (Variables|Movement|GetCurrentCell)) :!label _label)
            (Variables|/Game/Systems/BP_Gamestate.BP_Gamestate_C|SetIsActivePlayerMoving _asbp_gamestate true)
            (Audio|PlaySound2D "/Game/Assets/Audio/SFX/A_MovementPawn.A_MovementPawn" 1.0 1.0 0.0 0 0)
            (bind _movementevolution (Timeline|Timeline PlayFromStart)
              (:Update
                ;;[1 0.2292 0.5518] I know this is disgusting
                (bind _z (Timeline|Timeline_0 Play)
                  (:Update
                    (Transformation|SetActorLocation (Math|Vector|MakeVector (.X (Math|Vector|BreakVector (Math|Vector|Lerp(Vector) (Variables|Movement|GetStartPos) (Variables|Movement|GetEndPos) _movementevolution))) (.Y (Math|Vector|BreakVector (Math|Vector|Lerp(Vector) (Variables|Movement|GetStartPos) (Variables|Movement|GetEndPos) _movementevolution))) (+ (.Z (Math|Vector|BreakVector (Math|Vector|Lerp(Vector) (Variables|Movement|GetStartPos) (Variables|Movement|GetEndPos) _movementevolution))) (* _z 2e+02) 88.0)) false false))
                  (:Finished
                    (Timeline|Timeline_0 SetNewTime))))
              (:Finished
                (Math|Integer|DecrementInt (Variables|Movement|GetRemainingMovement)
                  (:%20%20
                    (Variables|TurnState|SetIsInPathChoice false)
                    (Variables|Movement|SetStartPos (Variables|Movement|GetEndPos))
                    (Timeline|Timeline_0 Stop)))))
            (else
              (bind _nextcell (Default|RequestNextCell (Variables|Movement|GetCurrentCell) (Variables|Movement|GetMoveBackwards)))
              (bind _output_get (Variables|Movement|SetCurrentCell _nextcell))
              (Utilities|IsValid _output_get
                (:Is%20Valid
                  (goto _label))
                (:Is%20Not%20Valid
                  (Variables|/Game/Systems/BP_Gamestate.BP_Gamestate_C|SetIsActivePlayerMoving _asbp_gamestate false)
                  (Variables|TurnState|SetIsInPathChoice true)))))))
      (elif (Variables|TurnState|GetHasUsedCell)
        (Variables|TurnState|SetIsActivePlayer false :!label _label_2)
        (Variables|TurnState|SetHasUsedDice false)
        (Variables|TurnState|SetHasUsedCell false)
        (Class|BPIPlayerRequestReceiver|RequestPlayerTurnEnd(Message) (Game|GetGameState))
        (goto _label_3 Reset)
        (else
          (Utilities|FlowControl|DoOnce false :!label _label_3
            (:Completed
              (Default|UseCell (Variables|Movement|GetCurrentCell)))))))
    (elif (and (Variables|Default|GetskipNextTurn) (Variables|TurnState|GetIsActivePlayer))
      (Variables|Default|SetskipNextTurn false)
      (goto _label_2))))

(fn ConstructionScript)