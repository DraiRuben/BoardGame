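; BP_Controller is a controller Blueprint that sets up player input and provides debug controls for the Talismans and Coins counters.
; On BeginPlay it adds the IMC_PlayerInputMap mapping context through the Enhanced Input local player subsystem.
; Two debug input actions, on Started, add their action value to the matching GameState counter and truncate the result to an integer.
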(event Input|EnhancedActionEvents|EnhancedInputActionIA_DebugCoins
  (params (ActionValue :type Float%20%28double-precision%29) (ElapsedSeconds :type Float%20%28double-precision%29) (TriggeredSeconds :type Float%20%28double-precision%29) (InputAction :type Input%20Action%20Object%20Reference :default "/Game/Inputs/IA_DebugCoins.IA_DebugCoins"))
  (bind _gamestate (CallFunction|GetGamestate))
  (:Started
    (Variables|/Game/Systems/BP_Gamestate.BP_Gamestate_C|SetCoins _gamestate (Math|Float|Truncate (+ (Variables|/Game/Systems/BP_Gamestate.BP_Gamestate_C|GetCoins _gamestate) ActionValue)))))

(event Input|EnhancedActionEvents|EnhancedInputActionIA_DebugTalismans
  (params (ActionValue :type Float%20%28double-precision%29) (ElapsedSeconds :type Float%20%28double-precision%29) (TriggeredSeconds :type Float%20%28double-precision%29) (InputAction :type Input%20Action%20Object%20Reference :default "/Game/Inputs/IA_DebugTalismans.IA_DebugTalismans"))
  (bind _gamestate (CallFunction|GetGamestate))
  (:Started
    (Variables|/Game/Systems/BP_Gamestate.BP_Gamestate_C|SetTalismans _gamestate (Math|Float|Truncate (+ (Variables|/Game/Systems/BP_Gamestate.BP_Gamestate_C|GetTalismans _gamestate) ActionValue)))))

(event EventBeginPlay
  (Input|AddMappingContext (PlayerController|LocalPlayerSubsystems|GetEnhancedInputLocalPlayerSubsystem) "/Game/Inputs/IMC_PlayerInputMap.IMC_PlayerInputMap" 0 "(bIgnoreAllPressedKeysUntilRelease=True,bForceImmediately=False,bNotifyUserSettings=False)"))

(fn ConstructionScript)