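; Game state Blueprint for a turn-based board game, tracking the player pawns, whose turn it is and a single Coins total.
; On BeginPlay it collects all BP_Pion actors and activates the first.
; A turn-end request toggles the moving flag around a one-second delay, then activates the next player with refilled movement, wrapping around.
; It also relays a path-choice-disabled call; RequestNextCell is an empty stub.
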(event EventBeginPlay
  (bind _outactors (Actor|GetAllActorsOfClass "/Game/Player/BP_Pion.BP_Pion_C"))
  (bind _output_get (Variables|Default|SetPlayers _outactors))
  (Variables|/Game/Player/BP_Pion.BP_Pion_C|SetisActivePlayer (Utilities|Array|Get(acopy) _output_get) true))

(event EventDisablePathChoice
  (Default|CallOnPathChoiceModeDisabled))

(event EventRequestPlayerTurnEnd
  ;[1 0 0.1406] Go to next turn, if we are back on the initial player then increase global turn
  (Variables|Default|SetIsActivePlayerMoving false)
  (Utilities|FlowControl|Delay 1.0)
  (Variables|Default|SetIsActivePlayerMoving true)
  (Math|Integer|IncrementInt (Variables|Default|GetCurrentPlayerTurn)
    (:%20%20
      (if (>= (Variables|Default|GetCurrentPlayerTurn) (Utilities|Array|Length (Variables|Default|GetPlayers)))
        (Variables|Default|SetCurrentPlayerTurn 0))
      (Variables|/Game/Player/BP_Pion.BP_Pion_C|SetremainingMovement (Utilities|Array|Get(acopy) (Variables|Default|GetPlayers) (Variables|Default|GetCurrentPlayerTurn)) 6)
      (Variables|/Game/Player/BP_Pion.BP_Pion_C|SetisActivePlayer (Utilities|Array|Get(acopy) (Variables|Default|GetPlayers) (Variables|Default|GetCurrentPlayerTurn)) true))))

(fn ConstructionScript)

(fn GetActivePlayer
  (return (Utilities|Array|Get(acopy) (Variables|Default|GetPlayers) (Variables|Default|GetCurrentPlayerTurn))))

(fn RequestCoinIncrease
  (params (IncreaseAmount :type Integer))
  (bind _output_get (Variables|Default|SetCoins (+ (Variables|Default|GetCoins) IncreaseAmount)))
  (return _output_get))

(fn RequestNextCell
  (return 0))