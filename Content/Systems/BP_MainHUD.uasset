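; BP_MainHUD creates and manages the UI widgets for a dice game.
; On BeginPlay it adds the main UI, dice roll, player count, main menu, dice bonus/malus and win menu widgets to the viewport.
; It keeps references to the main, dice and bonus/malus widgets in variables.
; The win menu starts collapsed and is made visible by the Win event.
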(event Custom|Win
  (Widget|SetVisibility (stale EventBeginPlay _returnvalue_7) "Visible"))

(event EventBeginPlay
  (bind _returnvalue (Game|GetPlayerController 0))
  (bind _returnvalue_2 (UserInterface|CreateWidget "/Game/Widgets/GameUI/WBP_MainUI.WBP_MainUI_C" (Game|GetPlayerController 0)))
  (Variables|Default|SetMainHUD _returnvalue_2)
  (bind _returnvalue_3 (UserInterface|CreateWidget "/Game/Widgets/Dice/WBP_RollDice.WBP_RollDice_C" _returnvalue))
  (UserInterface|Viewport|AddtoViewport _returnvalue_2 0)
  (Variables|Default|SetDiceHUD _returnvalue_3)
  (bind _returnvalue_4 (UserInterface|CreateWidget "/Game/Widgets/Menus/WBP_ChosePlayerNumber.WBP_ChosePlayerNumber_C" _returnvalue))
  (UserInterface|Viewport|AddtoViewport _returnvalue_4 0)
  (bind _returnvalue_5 (UserInterface|CreateWidget "/Game/Widgets/Menus/WBP_MainMenu.WBP_MainMenu_C" _returnvalue))
  (UserInterface|Viewport|AddtoViewport _returnvalue_5 0)
  (bind _returnvalue_6 (UserInterface|CreateWidget "/Game/Widgets/Dice/WBP_DiceBonusMalus.WBP_DiceBonusMalus_C" _returnvalue))
  (bind _output_get (Variables|Default|SetDiceBonusMalusHUD _returnvalue_6))
  (UserInterface|Viewport|AddtoViewport _output_get 0)
  (bind _returnvalue_7 (UserInterface|CreateWidget "/Game/Widgets/Menus/WBP_WinMenu.WBP_WinMenu_C"))
  (Widget|SetVisibility _returnvalue_7 "Collapsed")
  (UserInterface|Viewport|AddtoViewport _returnvalue_7 0))

(fn ConstructionScript)